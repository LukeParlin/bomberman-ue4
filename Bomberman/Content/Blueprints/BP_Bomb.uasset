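; Bomberman bomb actor that explodes after a short fixed fuse by destroying itself.
; Its Destroyed event passes player ID, explosion radius and tile coordinate to the Bomberman game mode's ExplodeBomb, so any destruction triggers the blast.
; When an actor's overlap with it ends, its sphere starts blocking pawns, letting the player step off before it becomes solid.
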(event EventBeginPlay
  ;[1 1 1] Bombs have a lifetime of 2 seconds. Then they explode.
  (Variables|Default|SetSpawnCollisionHandlingMethod "AlwaysSpawn") ; Spawn the bomb even inside a player!
  (Utilities|FlowControl|Delay 2.0)
  (Actor|DestroyActor))

(event EventDestroyed
  ;[1 1 1] When a bomb is destroyed, it calls the Explode Bomb function of BombermanGameMode
  (bind _asbp_bomberman_game_mode (Utilities|Casting|CastToBP_Bomberman_GameMode (Game|GetGameMode)))
  (Class|BombermanGameModeBase|ExplodeBomb _asbp_bomberman_game_mode (Variables|Default|GetplayerID) (Variables|Default|GetexplosionRadius) (Variables|Default|GettileCoord)))

(event Collision|EventActorEndOverlap
  (params (OtherActor :type Actor%20Object%20Reference))
  ;[1 1 1] Enable collision with the player AFTER they step off the bomb
  (Collision|SetCollisionResponsetoChannel (Variables|Default|GetSphere) "ECC_Pawn" "ECR_Block"))

(fn ConstructionScript)