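; BP_Bomberman is the Bomberman pawn, handling movement and facing from Player 1 input.
; Each Tick, GetMovementInput builds a flat world-space vector from the P1_Vertical and P1_Horizontal axes, which is then normalized.
; When that direction passes a length check, the actor snaps to face it and receives full-scale movement input along it.
; Because the check follows normalization, it filters only near-zero input rather than acting as an analog deadzone.
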(event EventTick
  (params (DeltaSeconds :type Float%20%28single-precision%29))
  (bind _returnvalue (Transformation|GetActorLocation))
  (bind _moveaxes (CallFunction|GetMovementInput))
  (bind _output_get (Variables|Default|SetDirection (Math|Vector|Normalize _moveaxes)))
  (if (> (Math|Vector|VectorLength _output_get) 0.2)
    (Transformation|SetActorRotation (Math|Rotator|FindLookatRotation _returnvalue (+ _returnvalue (Variables|Default|GetDirection))))
    (Pawn|Input|AddMovementInput (Math|Vector|Normalize _moveaxes) 1.0 false)))

(fn ConstructionScript)

(fn GetMovementInput
  (return (Math|Vector|MakeVector (Input|AxisValues|GetP1_Vertical) (Input|AxisValues|GetP1_Horizontal) 0.0)))