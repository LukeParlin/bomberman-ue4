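; Game mode for a two-player Bomberman game that spawns the HUD on BeginPlay and decides the match result.
; Tick runs the game countdown while both players live, declaring a draw on timeout.
; A death starts a short grace countdown so shared-blast kills count as a draw, then validity checks on Players pick the winner.
; Each result sets WinString, shows the win screen with UI-only input and resets both timers.
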(event EventBeginPlay
  ;[1 1 1] Spawn the HUD
  (bind _returnvalue (UserInterface|CreateWidget "/Game/Blueprints/BP_HUD.BP_HUD_C"))
  (UserInterface|Viewport|AddtoViewport _returnvalue 0))

(event EventTick
  (params (DeltaSeconds :type Float%20%28single-precision%29))
  (bind _players (Variables|Default|Getplayers))
  (bind _output (Utilities|Array|Get(acopy) _players))
  (bind _output_2 (Utilities|Array|Get(acopy) _players 1))
  (bind _returnvalue (Utilities|IsValid _output))
  (bind _returnvalue_2 (Utilities|IsValid _output_2))
  (bind _returnvalue_3 (not _returnvalue_2))
  (bind _returnvalue_4 (not _returnvalue))
  ;[1 1 1] Win condition check
  (if (== (Utilities|Array|Length _players) 2) ; If there are two players...
    (if (or _returnvalue_4 _returnvalue_3) ; ...and either one is dead
      ;[1 1 1] Only begin the win countdown timer after somebody dies
      (Variables|Default|SetWin%20Countdown (- (Variables|Default|GetWin%20Countdown) DeltaSeconds))
      (if (<= (Variables|Default|GetWin%20Countdown) 0.0)
        ;[1 1 1] Once the win countdown has finished, we can check who is dead and determine the winner
        (if (and _returnvalue_4 _returnvalue_3) ; Check if both players are dead
          (Variables|Default|SetWin%20String "It's a DRAW!")
          ;[1 1 1] Once we have determined our winner, create the win screen widget and give it input focus
          (bind _returnvalue_5 (UserInterface|CreateWidget "/Game/Blueprints/BP_WinScreen.BP_WinScreen_C" :!label _label))
          (UserInterface|Viewport|AddtoViewport _returnvalue_5 0)
          (Input|SetInputModeUIOnly (Game|GetPlayerController 0) _returnvalue_5 "DoNotLock")
          (Variables|Default|SetGame%20Countdown 1.2e+02) ; Reset the Game Countdown timer in case the game resets
          (Variables|Default|SetWin%20Countdown 0.2) ; Reset the Win Countdown timer in case the game resets
          (elif _returnvalue_4 ; Check if Red is dead
            (Variables|Default|SetWin%20String "BLUE is the winner!")
            (goto _label)
            (elif _returnvalue_3 ; Check if Blue is dead
              (Variables|Default|SetWin%20String "RED is the winner!")
              (goto _label)))))
      (else
        ;[1 1 1] Only decrement the game countdown timer while both players are alive
        (Variables|Default|SetGame%20Countdown (- (Variables|Default|GetGame%20Countdown) DeltaSeconds))
        (if (<= (Variables|Default|GetGame%20Countdown) 0.0)
          ;[1 1 1] If the game countdown finishes, the game ends in a draw
          (Variables|Default|SetWin%20String "TIme's up! It's a DRAW!")
          (goto _label))))))

(fn ConstructionScript)