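; BP_Explosion_Effect is a short-lived explosion effect actor that animates its scale and then removes itself.
; It starts at zero scale on BeginPlay, then each Tick accumulates elapsed time and samples ScaleCurve to set a uniform actor scale.
; Once elapsed time passes half a second, the actor destroys itself.
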(event EventBeginPlay
  (Transformation|SetActorScale3D "0, 0, 0"))

(event EventTick
  (params (DeltaSeconds :type Float%20%28single-precision%29))
  (bind _output_get (Variables|Default|SetElapsedTime (+ DeltaSeconds (Variables|Default|GetElapsedTime))))
  (Transformation|SetActorScale3D (* (Math|Vector|MakeVector 1.0 1.0 1.0) (Math|Curves|GetFloatValue (Variables|Default|GetScaleCurve) _output_get)))
  (if (> _output_get 0.5)
    (Actor|DestroyActor)))

(fn ConstructionScript)