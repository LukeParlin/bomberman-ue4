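; BP_Powerup is a powerup actor that plays a scale-in animation when play begins, with no pickup or effect logic of its own.
; BeginPlay sets the scale to zero, then Tick accumulates elapsed time and drives uniform scale from the ScaleCurve float curve.
; Once the short animation window ends, it snaps to full scale and disables its own tick.
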(event EventBeginPlay
  (Transformation|SetActorScale3D "0, 0, 0"))

(event EventTick
  (params (DeltaSeconds :type Float%20%28single-precision%29))
  (bind _output_get (Variables|Default|SetElapsed%20Time (+ DeltaSeconds (Variables|Default|GetElapsed%20Time))))
  (if (<= _output_get 0.8)
    (Transformation|SetActorScale3D (* (Math|Vector|MakeVector 1.0 1.0 1.0) (Math|Curves|GetFloatValue (Variables|Default|GetScale%20Curve) _output_get)))
    (else
      (Transformation|SetActorScale3D "1.000000,1.000000,1.000000")
      (Actor|Tick|SetActorTickEnabled false))))

(fn ConstructionScript)